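; Player-controlled marine pawn with world-axis movement, twin-stick-style aiming, rifle fire effects and health, which creates its HUD on BeginPlay.
; Each tick it sets control yaw from the thumbstick angle or smoothed mouse-movement direction, both deadzone-filtered, switching by the last key pressed.
; Firing here only toggles a muzzle-flash component and loop/end sounds, with no hit logic.
; Damage reduces health; at zero, Dead stops firing and blocks movement, aiming and shooting.
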(event `self.ReceiveBeginPlay`
  (bind _returnvalue (`|CreateWidget` "/Game/UI/W_PlayerHUD.W_PlayerHUD_C" null self))
  (`UserWidget.AddToViewport` _returnvalue 0))

(event `InputAxis|MoveForward`
  (params (AxisValue :type "Float (single-precision)"))
  (if (`self.Is Alive`)
    (`self.AddMovementInput` (1.0 0.0 0.0) AxisValue)))

(event `InputAction|Fire Weapon`
  (params (Key :type "Key Structure"))
  (:`Pressed`
    (`self.Start Fire Weapon`))
  (:`Released`
    (`self.Stop Fire Weapon`)))

(event `InputAxis|MoveRight`
  (params (AxisValue :type "Float (single-precision)"))
  (if (`self.Is Alive`)
    (`self.AddMovementInput` (0.0 1.0 0.0) AxisValue)))

(event `self.ReceiveTick`
  (params (DeltaSeconds :type "Float (single-precision)"))
  (if (`self.Is Alive`)
    (`self.Update Player Aim`)))

(event `Key|AnyKey`
  (params (Key :type "Key Structure"))
  (:`Pressed`
    (set `self.Gamepad Active` (`KismetInputLibrary.Key_IsGamepadKey` Key))))

(event `self.ReceiveAnyDamage`
  (params (Damage :type "Float (single-precision)") (DamageType :type "DamageType Object Reference") (InstigatedBy :type "Controller Object Reference") (DamageCauser :type "Actor Object Reference"))
  (bind _health (`self.Decrease Health` Damage))
  (if (== _health 0.0)
    (set `self.Dead` true)
    (`self.Stop Fire Weapon`)))

(fn `Decrease Health`
  (params (`Damage Amount` :type "Float (double-precision)"))
  (returns (Health :type "Float (double-precision)"))
  (bind _output_get (set `self.Health` (`KismetMathLibrary.FClamp` (- (`self.Health`) `Damage Amount`) 0.0 100.0)))
  (return _output_get))

(fn `Get Mouse Aim Direction`
  (returns (ReturnValue :type "Rotator Structure"))
  (bind (_returnvalue_x _returnvalue_y) (`KismetMathLibrary.BreakVector2D` (`self.Get Mouse Velocity`)))
  (return (`KismetMathLibrary.RInterpTo` (`Controller.GetControlRotation` (`GameplayStatics.GetPlayerController` 0)) (`KismetMathLibrary.MakeRotator` 0.0 0.0 (`KismetMathLibrary.DegAtan2` _returnvalue_x _returnvalue_y)) (`GameplayStatics.GetWorldDeltaSeconds`) (`self.Mouse Smoothing Strength`))))

(fn `Get Mouse Velocity`
  (returns (ReturnValue :type "Vector2D Structure"))
  (bind (_deltax _deltay) (`PlayerController.GetInputMouseDelta` (`GameplayStatics.GetPlayerController` 0)))
  (return (/ (`KismetMathLibrary.MakeVector2D` _deltax _deltay) (`GameplayStatics.GetWorldDeltaSeconds`))))

(fn `Get Thumbstick Aim Direction`
  (returns (ReturnValue :type "Rotator Structure"))
  (return (`KismetMathLibrary.MakeRotator` 0.0 0.0 (`KismetMathLibrary.DegAtan2` (`self.GetInputAxisValue`) (`self.GetInputAxisValue`)))))

(fn `Is Alive`
  (returns (ReturnValue :type Boolean))
  (return (not (`self.Dead`))))

(fn `Is Mouse Above Deadzone`
  (returns (ReturnValue :type Boolean))
  (return (> (`KismetMathLibrary.VSize2D` (`self.Get Mouse Velocity`)) (`self.MouseDeadzone`))))

(fn `Is Thumbstick Above Deadzone`
  (returns (ReturnValue :type Boolean))
  (return (> (`KismetMathLibrary.VSize2D` (`KismetMathLibrary.MakeVector2D` (`self.GetInputAxisValue`) (`self.GetInputAxisValue`))) (`self.ThumbstickDeadzone`))))

(fn `Start Fire Weapon`
  (if (`self.Is Alive`)
    (`ActorComponent.Activate` (`self.P_AssaultRifle_MF`) false)
    (bind _returnvalue (`GameplayStatics.SpawnSound2D` "/Game/Sounds/Weapon_AssaultRifle/Stereo/RifleFireLoop_Cue.RifleFireLoop_Cue" 1.0 1.0 0.0 null false false))
    (set `self.Weapon Fire Sond` _returnvalue)))

(fn `Stop Fire Weapon`
  (bind _weapon_fire_sond (`self.Weapon Fire Sond`))
  (`ActorComponent.Deactivate` (`self.P_AssaultRifle_MF`))
  (`/Engine/EditorBlueprintResources/StandardMacros.IsValid` _weapon_fire_sond
    (:`Is Valid`
      (`AudioComponent.Stop` _weapon_fire_sond)
      (if (`self.Is Alive`)
        (`GameplayStatics.SpawnSound2D` "/Game/Sounds/Weapon_AssaultRifle/Stereo/RifleFireEnd_Cue.RifleFireEnd_Cue" 1.0 1.0 0.0 null false false)))))

(fn `Update Mouse Aim`
  (if (`self.Is Mouse Above Deadzone`)
    (`Controller.SetControlRotation` (`GameplayStatics.GetPlayerController` 0) (`self.Get Mouse Aim Direction`))))

(fn `Update Player Aim`
  (if (`self.Gamepad Active`)
    (`self.Update Thumbstick Aim`)
    (else
      (`self.Update Mouse Aim`))))

(fn `Update Thumbstick Aim`
  (if (`self.Is Thumbstick Above Deadzone`)
    (`Controller.SetControlRotation` (`GameplayStatics.GetPlayerController` 0) (`self.Get Thumbstick Aim Direction`))))

(fn `UserConstructionScript`)